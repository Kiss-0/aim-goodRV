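; VR player pawn that grabs and throws BP_Ball actors and clicks on widgets through left and right widget interaction components.
; Grab snaps a ball overlapping GrabSphere to it with physics off; release detaches it, restores physics and adds a fixed world +X velocity.
; VR and PC trigger inputs press and release pointer keys, though the right VR trigger passes None instead of a mouse button.
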(event EventBeginPlay)

(event Collision|EventActorBeginOverlap
  (params (OtherActor :type Actor%20Object%20Reference)))

(event EventTick
  (params (DeltaSeconds :type Float%20%28single-precision%29)))

(event Input|ActionEvents|InputActionPC_Trigger_Left
  (params (Key :type Key%20Structure :default "None"))
  (bind _wi_left (Variables|Default|GetWI_Left))
  (:Pressed
    (Class|WidgetInteractionComponent|PressPointerKey _wi_left Key))
  (:Released
    (Class|WidgetInteractionComponent|ReleasePointerKey _wi_left Key)))

(event Input|ActionEvents|InputActionVR_Trigger_Right
  (params (Key :type Key%20Structure :default "None"))
  (bind _wi_right (Variables|Default|GetWI_Right))
  (:Pressed
    (Class|WidgetInteractionComponent|PressPointerKey _wi_right "None"))
  (:Released
    (Class|WidgetInteractionComponent|ReleasePointerKey _wi_right "None")))

(event Input|ActionEvents|InputActionIA_Grab
  (params (Key :type Key%20Structure :default "None"))
  (:Pressed
    (for _array_element (Collision|GetOverlappingActors (Variables|Default|GetGrabSphere) "/Game/BluePrints/BP_Ball.BP_Ball_C" :!class /Script/Engine.PrimitiveComponent)
      (bind _asbp_ball (Utilities|Casting|CastToBP_Ball _array_element))
      (bind _output_get (Variables|Default|SetObjetoAgarrado _asbp_ball))
      (Physics|SetSimulatePhysics (Variables|/Game/BluePrints/BP_Ball.BP_Ball_C|GetCube _output_get) false)
      (Transformation|AttachComponentToComponent (Variables|Default|GetObjetoAgarrado) (Variables|Default|GetGrabSphere) "None" "SnapToTarget" "SnapToTarget" "KeepRelative" true)))
  (:Released
    (Utilities|IsValid (Variables|Default|GetObjetoAgarrado)
      (:Is%20Valid
        (Transformation|DetachFromActor (Variables|Default|GetObjetoAgarrado) "KeepRelative" "KeepRelative" "KeepRelative")
        (Physics|SetSimulatePhysics (Variables|/Game/BluePrints/BP_Ball.BP_Ball_C|GetCube (Variables|Default|GetObjetoAgarrado)) true)
        (Physics|SetPhysicsLinearVelocity (Variables|/Game/BluePrints/BP_Ball.BP_Ball_C|GetCube (Variables|Default|GetObjetoAgarrado)) "100.000000,0.000000,0.000000" true "None")
        (Variables|Default|SetObjetoAgarrado 0)))))

(event Input|ActionEvents|InputActionVR_Trigger_Left
  (params (Key :type Key%20Structure :default "None"))
  (bind _wi_left (Variables|Default|GetWI_Left))
  (:Pressed
    (Class|WidgetInteractionComponent|PressPointerKey _wi_left "LeftMouseButton"))
  (:Released
    (Class|WidgetInteractionComponent|ReleasePointerKey _wi_left "LeftMouseButton")))

(fn ConstructionScript)